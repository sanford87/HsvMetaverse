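; BP_CameraViz visualizes a recorded series of camera positions and orientations as static meshes in the level.
; The construction script adds one mesh per array entry, with scaled position and per-axis rotation multipliers, and stores each resulting world transform.
; On Tick, a cube eases toward the raw location entry indexed by whole seconds of game time, without using the stored world transforms or wrapping the index.
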(event `self.ReceiveBeginPlay`
  (set `self.VideoLength` (`KismetArrayLibrary.Array_Length` (`self.CameraLocationArray`))))

(event `self.ReceiveTick`
  (params (DeltaSeconds :type "Float (single-precision)"))
  (`SceneComponent.K2_SetWorldLocationAndRotation` :`self` (`self.Cube`) :`NewLocation` (`KismetMathLibrary.VInterpTo` (`SceneComponent.RelativeLocation` (`self.Cube`)) (`|GetArrayItem` (`self.CameraLocationArray`) (`KismetMathLibrary.FFloor` (`KismetSystemLibrary.GetGameTimeInSeconds`))) DeltaSeconds 1.0)))

(fn `UserConstructionScript`
  ;[1 1 1] Set Camera image location
  (for (_array_element _array_index) (`self.CameraLocationArray`)
    (bind _returnvalue (`AddComponent|NODE_AddStaticMeshComponent-0` :`RelativeTransform` (`KismetMathLibrary.MakeTransform` (* (`self.PositionScale`) _array_element) (`KismetMathLibrary.MakeRotator` (* (.roll (`|GetArrayItem` (`self.CameraOrientationArray`) _array_index)) (`self.xMod`)) (* (.pitch (`|GetArrayItem` (`self.CameraOrientationArray`) _array_index)) (`self.yMod`)) (* (.yaw (`|GetArrayItem` (`self.CameraOrientationArray`) _array_index)) (`self.zMod`))) (`KismetMathLibrary.Conv_DoubleToVector` (`self.Scale`)))))
    (`KismetArrayLibrary.Array_Add` (`self.CameraLocationArray_World`) (`SceneComponent.K2_GetComponentLocation` _returnvalue))
    (`KismetArrayLibrary.Array_Add` (`self.CameraOrientationArray_World`) (`SceneComponent.K2_GetComponentRotation` _returnvalue))))