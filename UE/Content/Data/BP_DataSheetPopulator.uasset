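; BP_DataSheetPopulator turns data table rows into camera transforms for BP_CameraViz, working entirely in its construction script.
; A FillArray helper reads each position and rotation column as strings and converts them to numeric arrays.
; These are combined per index into scaled location vectors and rotators.
; Both resulting arrays are then copied onto the BP_CameraViz actor found with GetActorOfClass.
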(fn `UserConstructionScript`
  (bind _xarray (`self.xArray`))
  (`|ExecutionSequence`
    (:`then_0`
      (`self.FillArray` "x" (`self.xArray`)
        (:`Out`
          (`self.FillArray` "y" (`self.yArray`)
            (:`Out`
              (`self.FillArray` "z" (`self.zArray`)
                (:`Out`
                  (`self.FillArray` "Yaw" (`self.yawArray`)
                    (:`Out`
                      (`self.FillArray` "pitch" (`self.pitchArray`)
                        (:`Out`
                          (`self.FillArray` "roll" (`self.rollArray`)
                            (:`Out`
                              (for (_ _array_index) _xarray
                                (`KismetArrayLibrary.Array_Set` (`self.CameraLocationArray`) _array_index (* (`self.PositionScale`) (`KismetMathLibrary.MakeVector` (`|GetArrayItem` _xarray _array_index) (`|GetArrayItem` (`self.yArray`) _array_index) (`|GetArrayItem` (`self.zArray`) _array_index))) true)
                                (`KismetArrayLibrary.Array_Set` (`self.CameraOrientationArray`) _array_index (`KismetMathLibrary.MakeRotator` (`|GetArrayItem` (`self.rollArray`) _array_index) (`|GetArrayItem` (`self.pitchArray`) _array_index) (`|GetArrayItem` (`self.yawArray`) _array_index)) true)))))))))))))))
    (:`then_1`
      (bind _returnvalue (`GameplayStatics.GetActorOfClass` "/Game/Data/BP_CameraViz.BP_CameraViz_C"))
      (set `/Game/Data/BP_CameraViz.CameraLocationArray` (`self.CameraLocationArray`) _returnvalue)
      (set `/Game/Data/BP_CameraViz.CameraOrientationArray` (`self.CameraOrientationArray`) _returnvalue))))