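; Streaming test Blueprint for trying video sources on a Media Player; despite its name, it spawns no widget.
; On BeginPlay it only passes TestVideo_02 to SetMediaOptions, with no open or play call connected.
; Disconnected experiments cover enumerated webcam capture, a hard-coded capture device, a TestVideo source, manual Play, Amazon IVS HLS and ARN addresses, and a YouTube embed string.
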(event `self.ReceiveBeginPlay`
  (`MediaPlayer.SetMediaOptions` (`self.MediaPlayer`) "/Game/Movies/TestVideo_02.TestVideo_02"))

(fn `UserConstructionScript`)