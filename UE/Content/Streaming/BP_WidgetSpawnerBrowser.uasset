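; Streaming test Blueprint, named as a browser widget spawner, that holds experiments in feeding video to a Media Player.
; BeginPlay and the construction script are empty, and every media node is disconnected, so none of this logic runs.
; The unused snippets try a TestVideo media source, the first enumerated webcam, YouTube embed URLs and a hard-coded USB capture device URL.
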(event `self.ReceiveBeginPlay`)

(fn `UserConstructionScript`)