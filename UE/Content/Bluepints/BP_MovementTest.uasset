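; BP_MovementTest is a test Blueprint that moves a Cube component through the locations in PointArray over game time.
; After a three-second delay on BeginPlay, it stores a time offset and starts a looping timer that interpolates the cube toward the point indexed by elapsed whole seconds.
; Speed sets both timer interval and interpolation speed.
; The construction script prints the names of BPCameraViz's child actors.
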(event `self.ReceiveBeginPlay`
  (`KismetSystemLibrary.Delay` 3.0)
  (set `self.TimeStampOffset` (`KismetMathLibrary.FFloor` (`KismetSystemLibrary.GetGameTimeInSeconds`)))
  (set `self.PointArrayLength` (`KismetArrayLibrary.Array_Length` (`self.PointArray`)))
  (`KismetSystemLibrary.K2_SetTimerDelegate` (delegate `UpdatePoint`) (`self.Speed`) true))

(event `self.ReceiveTick`
  (params (DeltaSeconds :type "Float (single-precision)")))

(event `UpdatePoint`
  (if (< (`self.GetLocalTime`) (`self.PointArrayLength`))
    (`SceneComponent.K2_SetWorldLocation` (`self.Cube`) (`KismetMathLibrary.VInterpTo` (`SceneComponent.K2_GetComponentLocation` (`self.Cube`)) (`|GetArrayItem` (`self.PointArray`) (`self.GetLocalTime`)) 1.0 (`self.Speed`)) false false)))

(fn `GetLocalTime`
  (returns (TimeIncement :type Integer))
  (return (- (`KismetMathLibrary.FFloor` (`KismetSystemLibrary.GetGameTimeInSeconds`)) (`self.TimeStampOffset`))))

(fn `UserConstructionScript`
  (for _array_element (`self.GetAllChildActors` (`self.BP_CameraViz`) true)
    (`KismetSystemLibrary.PrintString` (`KismetSystemLibrary.GetDisplayName` _array_element))))