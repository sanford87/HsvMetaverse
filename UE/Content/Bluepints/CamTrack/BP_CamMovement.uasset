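; Camera actor that moves a scene capture component along recorded location and rotation arrays, indexed by whole seconds of game time.
; A looping timeline lerps from the current second's sample to the next, re-reading the index on each finish without a bounds check.
; The construction script snaps to the first sample and sets FOV.
; Video playback, time-offset setup and an older interpolation approach are disconnected.
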(event `self.ReceiveBeginPlay`
  (bind _timeincement (`self.GetLocalTime`))
  (bind _camlocationarray (`self.CamLocationArray`))
  (bind _camrotationarray (`self.CamRotationArray`))
  (bind _returnvalue (+ _timeincement 1))
  (set `self.CurrentPoint` (`|GetArrayItem` _camlocationarray _timeincement) :!label _label)
  (set `self.CurrentRotation` (`|GetArrayItem` _camrotationarray _timeincement))
  (set `self.NextPoint` (`|GetArrayItem` _camlocationarray _returnvalue))
  (set `self.NextRotation` (`|GetArrayItem` _camrotationarray _returnvalue))
  (bind (_direction _newtrack_0) (`Timeline|Transition` :!via `PlayFromStart`)
    (:`Update`
      (`self.K2_SetActorLocationAndRotation` (`KismetMathLibrary.VLerp` (`self.CurrentPoint`) (`self.NextPoint`) _newtrack_0) (`KismetMathLibrary.RLerp` (`self.CurrentRotation`) (`self.NextRotation`) _newtrack_0)))
    (:`Finished`
      (goto _label))))

(event `self.ReceiveTick`
  (params (DeltaSeconds :type "Float (single-precision)")))

(event `UpdatePoint`)

(fn `GetLocalTime`
  (returns (TimeIncement :type Integer))
  (return (- (`KismetMathLibrary.FFloor` (`KismetSystemLibrary.GetGameTimeInSeconds`)) (`self.TimeStampOffset`))))

(fn `UserConstructionScript`
  (`self.K2_SetActorLocationAndRotation` (`|GetArrayItem` (`self.CamLocationArray`)) (`|GetArrayItem` (`self.CamRotationArray`)))
  (set `SceneCaptureComponent2D.FOVAngle` (`self.FieldOfView`) (`self.SceneCaptureComponent2D`)))